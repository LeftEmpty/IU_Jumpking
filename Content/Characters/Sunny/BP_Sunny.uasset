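; BP_Sunny is the Sunny character Blueprint, handling the screen feedback for death, respawn and victory.
; On BeginPlay it binds handlers to its OnDeath and OnVictory dispatchers.
; Death shows either an animated game over widget or a temporary respawn transition that is removed after a delay, depending on the GameOver flag.
; Victory waits briefly, then shows an animated victory screen.
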(event Custom|OnVictory_Event
  (params (Player :type J%20Character%20Object%20Reference))
  ;[1 1 1] Victory Screen
  (Utilities|FlowControl|Delay 2.0)
  (bind _returnvalue (UserInterface|CreateWidget "/Game/Blueprints/Widgets/WBP_Victory.WBP_Victory_C"))
  (bind _output_get (Variables|Default|SetVictoryScreen _returnvalue))
  (UserInterface|Viewport|AddtoViewport _output_get 0)
  (Default|PlayAnim (Variables|Default|GetVictoryScreen)))

(event Custom|OnDeath_Event
  (params (Player :type J%20Character%20Object%20Reference) (bGameOver :type Boolean))
  (if bGameOver
    ;[1 1 1] Game Over Screen
    (bind _returnvalue (UserInterface|CreateWidget "/Game/Blueprints/Widgets/WBP_GameOver.WBP_GameOver_C"))
    (bind _output_get (Variables|Default|SetGameOverScreen _returnvalue))
    (UserInterface|Viewport|AddtoViewport _output_get 0)
    (Default|PlayAnim (Variables|Default|GetGameOverScreen))
    (else
      ;[1 1 1] Respawn Transition
      (bind _returnvalue_2 (UserInterface|CreateWidget "/Game/Blueprints/Widgets/WBP_DeathTransition.WBP_DeathTransition_C"))
      (bind _output_get_2 (Variables|Default|SetRespawnTransition _returnvalue_2))
      (UserInterface|Viewport|AddtoViewport _output_get_2 0)
      (Default|PlayAnim (Variables|Default|GetRespawnTransition))
      (Utilities|FlowControl|Delay 3.0)
      (Widget|RemovefromParent (Variables|Default|GetRespawnTransition)))))

(event EventBeginPlay
  (EventDispatchers|AssignOnDeath (delegate Custom|OnDeath_Event))
  (EventDispatchers|AssignOnVictory (delegate Custom|OnVictory_Event)))

(event Collision|EventActorBeginOverlap
  (params (OtherActor :type Actor%20Object%20Reference)))

(event EventTick
  (params (DeltaSeconds :type Float%20%28single-precision%29)))

(fn ConstructionScript)