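; BP_PickUpBase is a platformer pickup, named as a base class, that destroys itself when any actor overlaps it.
; The construction script throttles the tick interval, and Tick is set up to apply a stepped yaw spin whenever the Second counter reaches a threshold.
; As written, Tick adds zero to Second, so the threshold is never reached and the spin does not fire.
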(event EventBeginPlay)

(event Collision|EventActorBeginOverlap
  (params (OtherActor :type Actor%20Object%20Reference))
  (Actor|DestroyActor))

(event EventTick
  (params (DeltaSeconds :type Float%20%28single-precision%29))
  (bind _output_get (Variables|Default|SetSecond (+ (Variables|Default|GetSecond) 0.0)))
  (if (>= _output_get 0.12)
    (Transformation|AddActorLocalRotation "0.000000,11.000000,0.000000" false false)
    (Variables|Default|SetSecond 0.0)))

(fn ConstructionScript
  (Actor|Tick|SetActorTickInterval 0.02))