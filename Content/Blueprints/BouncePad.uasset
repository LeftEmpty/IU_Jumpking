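; Bounce pad that bounces the player character off its surface.
; Overlapping the Collide volume saves the player's velocity before impact.
; A hit on the Cube reflects that saved velocity about the surface normal and launches player 0 with it, overriding both horizontal and vertical movement.
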(event OnComponentBeginOverlap(Collide)
  (params (OverlappedComponent :type Primitive%20Component%20Object%20Reference) (OtherActor :type Actor%20Object%20Reference) (OtherComp :type Primitive%20Component%20Object%20Reference) (OtherBodyIndex :type Integer) (bFromSweep :type Boolean) (SweepResult :type Hit%20Result%20Structure%20%28by%20ref%29))
  ;[1 1 1] If character enters collision box, save his movement Vector.
  (Variables|Default|SetVelocity (|GetPlayerVelocity)))

(event OnComponentHit(Cube)
  (params (HitComponent :type Primitive%20Component%20Object%20Reference) (OtherActor :type Actor%20Object%20Reference) (OtherComp :type Primitive%20Component%20Object%20Reference) (NormalImpulse :type Vector :default "0, 0, 0") (Hit :type Hit%20Result%20Structure%20%28by%20ref%29))
  ;[1 1 1] If the bouncepad is hit, the velocity is reflected on the surface of the pad.
  (Character|LaunchCharacter (Game|GetPlayerCharacter 0) (Math|Vector|GetReflectionVector (Variables|Default|GetVelocity) (|HitStruct Hit)) true true))

(fn ConstructionScript)