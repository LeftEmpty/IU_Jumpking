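; Log obstacle projectile that travels along a spline it is given.
; On BeginPlay it binds to OnSplineReceived, then validates the spline reference, printing an error if none is valid.
; A Timeline, with play rate scaled by TimelineLength, maps its alpha to distance along the spline, setting world location and aligning rotation to the tangent.
; The DestroyActor call is disconnected, so the log is not destroyed here.
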(event Custom|Play%20Timeline
  (bind _splineref (Variables|Default|GetSplineRef))
  (bind _alpha (Timeline|Timeline Play)
    (:Update
      (Transformation|SetActorLocationAndRotation (Spline|GetLocationatDistanceAlongSpline _splineref (Math|Float|Lerp 0.0 (Spline|GetSplineLength (Variables|Default|GetSplineRef)) _alpha) "World") (Math|Conversions|RotationFromXVector (Spline|GetTangentatDistanceAlongSpline _splineref (Math|Float|Lerp 0.0 (Spline|GetSplineLength (Variables|Default|GetSplineRef)) _alpha) "World"))))))

(event Custom|OnSplineReceived_Event
  (params (SplineRef :type Spline%20Component%20Object%20Reference))
  (bind _returnvalue (Class|JProjectileSpline|GetSplineReference))
  (Utilities|IsValid _returnvalue
    (:Is%20Valid
      (Variables|Default|SetSplineRef _returnvalue)
      (Components|Timeline|SetPlayRate (Variables|Default|GetTimeline) (/ 1.0 (Variables|Default|GetTimeline%20Length)))
      (CallFunction|PlayTimeline))
    (:Is%20Not%20Valid
      (Development|PrintString "Error: No valid spline reference provided"))))

(event EventBeginPlay
  (EventDispatchers|AssignOnSplineReceived (delegate Custom|OnSplineReceived_Event)))

(fn ConstructionScript)