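; BP_Hammer is a moving obstacle that swings back and forth between two rotation apexes.
; Construction stores the placed rotation as the start apex and, unless overridden, negates it for the end apex.
; BeginPlay scales the Timeline's play rate by TimelineLength, then PlayTimeline alternates the target apex after a delay at each end.
; Timeline updates lerp from the current rotation, not a fixed start, toward that target.
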(event Custom|Play%20Timeline
  (params (bAtStart :type Boolean))
  (if bAtStart
    (Variables|Default|SetMoveToRot (Variables|Default|GetEndRotationApex))
    (bind _alpha (Timeline|Timeline PlayFromStart)
      (:Update
        (Transformation|SetActorRotation (Math|Rotator|Lerp(Rotator) (Transformation|GetActorRotation) (Variables|Default|GetMoveToRot) _alpha)))
      (:Finished
        (Utilities|FlowControl|Delay (Variables|Default|GetDelayAtApex))
        (CallFunction|PlayTimeline (not bAtStart))))
    (else
      (Variables|Default|SetMoveToRot (Variables|Default|GetStartRotationApex))
      (Timeline|Timeline PlayFromStart))))

(event EventBeginPlay
  (Components|Timeline|SetPlayRate (Variables|Default|GetTimeline) (/ 1.0 (Variables|Default|GetTimeline%20Length)))
  (CallFunction|PlayTimeline true))

(event Collision|EventActorBeginOverlap
  (params (OtherActor :type Actor%20Object%20Reference)))

(event EventTick
  (params (DeltaSeconds :type Float%20%28single-precision%29)))

(fn ConstructionScript
  (bind _returnvalue (Transformation|GetActorRotation))
  (Variables|Default|SetStartRotationApex _returnvalue)
  (Variables|Default|SetMoveToRot _returnvalue)
  (if (not (Variables|Default|GetbOverwriteDefaultEndApex))
    (Variables|Default|SetEndRotationApex (* (Variables|Default|GetStartRotationApex) -1.0))))