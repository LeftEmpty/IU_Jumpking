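; Swinging hammer obstacle that rotates back and forth between two apex rotations, pausing at each.
; A timeline, rate-scaled by TravelTime, lerps from the current rotation toward the active target, then flips direction after DelayAtApex.
; Unless overwritten, construction takes the placed rotation as start and negates its RotationAxis component for the end.
; ChangeCollision can shrink or restore the death capsule, but its event-graph calls are unconnected.
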(event Custom|Play%20Timeline
  (params (AtStart :type Boolean))
  (if AtStart
    (Variables|Rotations|SetCurMoveToRot (Variables|Rotations|GetEndApexRot))
    (bind _alpha (Timeline|Timeline PlayFromStart)
      (:Update
        (Transformation|SetActorRotation (Math|Rotator|Lerp(Rotator) (Transformation|GetActorRotation) (Variables|Rotations|GetCurMoveToRot) _alpha)))
      (:Finished
        (Utilities|FlowControl|Delay (Variables|Default|GetDelayAtApex))
        (CallFunction|PlayTimeline (not AtStart))))
    (else
      (Variables|Rotations|SetCurMoveToRot (Variables|Rotations|GetStartApexRot))
      (Timeline|Timeline PlayFromStart))))

(event EventBeginPlay
  (Components|Timeline|SetPlayRate (Variables|Default|GetTimeline) (/ 1.0 (Variables|Default|GetTravelTime)))
  (CallFunction|PlayTimeline true))

(fn ConstructionScript
  (bind _returnvalue (Transformation|GetActorRotation))
  (bind _jdeathcollision (Variables|Default|GetJDeathCollision))
  (Utilities|FlowControl|Sequence
    (:then_0
      (Variables|Default|SetDeathCapsule%20Radius (Variables|/Script/Engine.CapsuleComponent|GetCapsuleRadius _jdeathcollision))
      (Variables|Default|SetDeathCapsule%20Half%20Height (Variables|/Script/Engine.CapsuleComponent|GetCapsuleHalfHeight _jdeathcollision)))
    (:then_1
      (if (not (Variables|Default|GetbOverwriteDefaultApex))
        (Variables|Rotations|SetStartApexRot _returnvalue)
        (Variables|Rotations|SetCurMoveToRot _returnvalue)
        (switch Utilities|FlowControl|Switch|SwitchonEAxis (Variables|Default|GetRotationAxis)
          (:None
            (Development|PrintString "ERROR setting default apex' on hammer"))
          (:X
            (Variables|Rotations|SetEndApexRot (Math|Rotator|MakeRotator (* (.roll (Variables|Rotations|GetStartApexRot)) -1.0) (.pitch (Variables|Rotations|GetStartApexRot)) (.yaw (Variables|Rotations|GetStartApexRot)))))
          (:Y
            (Variables|Rotations|SetEndApexRot (Math|Rotator|MakeRotator (.roll (Variables|Rotations|GetStartApexRot)) (* (.pitch (Variables|Rotations|GetStartApexRot)) -1.0) (.yaw (Variables|Rotations|GetStartApexRot)))))
          (:Z
            (Variables|Rotations|SetEndApexRot (Math|Rotator|MakeRotator (.roll (Variables|Rotations|GetStartApexRot)) (.pitch (Variables|Rotations|GetStartApexRot)) (* (.yaw (Variables|Rotations|GetStartApexRot)) -1.0)))))))))

(fn ChangeCollision
  (params (bTurnOn :type Boolean))
  (if bTurnOn
    (Components|Capsule|SetCapsuleRadius (Variables|Default|GetJDeathCollision) (Variables|Default|GetDeathCapsule%20Radius) true)
    (Components|Capsule|SetCapsuleHalfHeight (Variables|Default|GetJDeathCollision) (Variables|Default|GetDeathCapsule%20Half%20Height) true)
    (else
      (Components|Capsule|SetCapsuleRadius (Variables|Default|GetJDeathCollision) 1.0 true)
      (Components|Capsule|SetCapsuleHalfHeight (Variables|Default|GetJDeathCollision) 1.0 true))))