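; BP_SpikeField is an obstacle actor that lays out a rectangular grid of spike static meshes.
; The construction script loops over Rows and Columns, adding one static mesh component per cell, spaced by SpikeOffset in X and Y and scaled by SpikeScale.
; The event graph holds only disabled default events, so the Blueprint adds no runtime logic such as overlap handling or damage.
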(event EventBeginPlay)

(event Collision|EventActorBeginOverlap
  (params (OtherActor :type Actor%20Object%20Reference)))

(event EventTick
  (params (DeltaSeconds :type Float%20%28single-precision%29)))

(fn ConstructionScript
  (for _index (range 0 (- (Variables|Default|GetRows) 1))
    (for _index_2 (range 0 (- (Variables|Default|GetColumns) 1))
      (AddComponent|AddStaticMeshComponent false (Math|Transform|MakeTransform (Math|Vector|MakeVector (* (Math|Conversions|ToFloat(Integer) _index) (Variables|Default|GetSpikeOffset)) (* (Math|Conversions|ToFloat(Integer) _index_2) (Variables|Default|GetSpikeOffset)) 0.0) "0, 0, 0" (Variables|Default|GetSpikeScale))))))