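; Merry-go-round obstacle Blueprint meant to cycle a set of projectiles around a looping spline, though the graph spawns none itself.
; A self-restarting timeline, rate-scaled by TimelineLength, converts alpha to spline distance for each projectile, wrapping past the end.
; The movement is unfinished: the per-projectile offset is multiplied by zero, and the spline location and rotation lookups are not connected to the transform call.
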(event Custom|Play%20Timeline
  (bind _spline (Variables|Default|GetSpline))
  (bind _returnvalue (Spline|GetSplineLength _spline))
  (bind _alpha (Timeline|Timeline Play)
    (:Update
      (for _array_element (Variables|Default|GetProjectiles)
        (bind _output_get (Variables|Default|SetDistance%20Along%20Spline (+ (* 0.0 (Variables|Default|GetProjectile%20Offset)) (Math|Float|Lerp 0.0 (Spline|GetSplineLength (Variables|Default|GetSpline)) _alpha))))
        (if (> _output_get _returnvalue)
          (Variables|Default|SetDistance%20Along%20Spline (- (Variables|Default|GetDistance%20Along%20Spline) _returnvalue))
          (else
            (Transformation|SetActorLocationAndRotation "0, 0, 0" "0, 0, 0")))))
    (:Finished
      (CallFunction|PlayTimeline))))

(event EventBeginPlay
  (Components|Timeline|SetPlayRate (Variables|Default|GetTimeline) (/ 1.0 (Variables|Default|GetTimeline%20Length)))
  (CallFunction|PlayTimeline))

(fn ConstructionScript)