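; BP_DeathBox is a hazard actor that damages the Sunny player character on overlap and sends it back to a checkpoint.
; An overlap with BP_Sunny disables player movement and calls OnTakeDamage on the character.
; After a short delay it calls OnRespawn, then teleports the controlled pawn to the LastCheckpoint actor's location with zero rotation.
; Movement is not re-enabled in this Blueprint.
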(event EventBeginPlay)

(event EventTick
  (params (DeltaSeconds :type Float%20%28single-precision%29)))

(event Collision|EventActorBeginOverlap
  (params (OtherActor :type Actor%20Object%20Reference))
  (bind _asbp_sunny (Utilities|Casting|CastToBP_Sunny OtherActor))
  (Variables|Default|SetPlayer _asbp_sunny)
  (Pawn|Components|CharacterMovement|DisableMovement (Variables|/Script/Engine.Character|GetCharacterMovement (Game|GetPlayerCharacter 0)))
  (Class|JCharacter|OnTakeDamage (Variables|Default|GetPlayer))
  (Utilities|FlowControl|Delay 2.0)
  (Class|JCharacter|OnRespawn (Variables|Default|GetPlayer))
  (Transformation|Teleport (Pawn|GetControlledPawn (Game|GetPlayerController 0)) (Transformation|GetActorLocation (Variables|Default|GetLastCheckpoint)) "0, 0, 0"))

(fn ConstructionScript)